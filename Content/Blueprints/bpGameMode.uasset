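; Game mode that spawns a grid of BpEnemy actors at BeginPlay and keeps them in an Enemies array.
; Nested loops place each enemy at a fixed height, offsetting X and Y from start positions by index times XDistance and YDistance.
; A disconnected cleanup loop would destroy and remove hit enemies; Tick is empty, and a Norwegian note says deletion errored and temporarily moved to bpBullet.
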(event EventBeginPlay
  (for _index (range 0 6)
    (for _index_2 (range 0 4)
      (bind _output_get (Variables|Default|SetInitialSpawnLocation (Math|Vector|MakeVector (|((Index*Distance)+StartPosition) (Math|Conversions|ToFloat(Integer) _index) (Variables|Default|GetXDistance) 5e+02) (|((Index*Distance)+StartPosition) (Math|Conversions|ToFloat(Integer) _index_2) (Variables|Default|GetYDistance) -5e+02) 112.0)))
      (bind _returnvalue (Game|SpawnActorfromClass "/Game/Blueprints/bpEnemy.bpEnemy_C" (Math|Transform|MakeTransform _output_get "0, 0, 0" "1,1,1") "Undefined" 0 0))
      (Utilities|Array|Add (Variables|Default|GetEnemies) _returnvalue))))

(event EventTick
  (params (DeltaSeconds :type Float%20%28single-precision%29))
  ;[1 1 1] Er noe galt her. Får opp sykt mange error meldinger. Skal egentlig slette fiendene, men fungerer ikke, så gjør det i bpBullet istedet foreløpig
)

(fn ConstructionScript)