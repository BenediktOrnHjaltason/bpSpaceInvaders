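; Player pawn Blueprint that moves along world axes, shoots limited ammo and loses lives on contact with enemies.
; Overlapping a bpEnemy decrements Lives, then either pauses the game when none remain or teleports the player to InitialSpawnLocation, briefly hidden with collision and movement disabled.
; Shooting spawns a BpBullet at the SpawnLocation component while Ammo remains, then uses a Delay to destroy it.
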(event `self.ReceiveActorBeginOverlap`
  (params (OtherActor :type "Actor Object Reference"))
  (cast `/Game/Blueprints/bpEnemy` OtherActor)
  (bind _result (`/Engine/EditorBlueprintResources/StandardMacros.DecrementInt` (`self.Lives`))
    (:`  `
      (`/Engine/EditorBlueprintResources/StandardMacros.CompareInt` _result
        (:`>`
          (`PrimitiveComponent.SetCollisionEnabled` (`self.CapsuleComponent`) "NoCollision")
          (`self.SetActorHiddenInGame` true)
          (`SceneComponent.K2_SetWorldLocation` (`self.CapsuleComponent`) (`self.InitialSpawnLocation`) false false)
          (set `self.DisableMovement` true)
          (`KismetSystemLibrary.Delay` 1.0)
          (`self.SetActorHiddenInGame` false)
          (set `self.DisableMovement` false)
          (`PrimitiveComponent.SetCollisionEnabled` (`self.CapsuleComponent`) "QueryAndPhysics"))
        (:`==`
          (`GameplayStatics.SetGamePaused` true :!label _label))
        (:`<`
          (goto _label))))))

(event `InputAxis|MoveForward`
  (params (AxisValue :type "Float (single-precision)"))
  (if (not (`self.DisableMovement`))
    (`self.AddMovementInput` (1.0 0.0 0.0) AxisValue)))

(event `InputAxis|MoveRight`
  (params (AxisValue :type "Float (single-precision)"))
  (if (not (`self.DisableMovement`))
    (`self.AddMovementInput` (0.0 1.0 0.0) AxisValue)))

(event `InputAction|Shoot`
  (params (Key :type "Key Structure"))
  (:`Pressed`
    (`/Engine/EditorBlueprintResources/StandardMacros.CompareInt` (`self.Ammo`)
      (:`>`
        (bind _returnvalue (`|SpawnActorFromClass` "/Game/Blueprints/bpBullet.bpBullet_C" (`SceneComponent.K2_GetComponentToWorld` (`self.SpawnLocation`)) "AlwaysSpawn" "OverrideRootScale" null null))
        (`/Engine/EditorBlueprintResources/StandardMacros.DecrementInt` (`self.Ammo`)
          (:`  `
            (`KismetSystemLibrary.Delay` 4.0)
            (`self.K2_DestroyActor` _returnvalue)))))))

(fn `UserConstructionScript`)