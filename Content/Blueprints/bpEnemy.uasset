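; Enemy actor that moves along local X at its movement speed while zigzagging on Y.
; Tick scales both offsets by delta time, but a per-frame counter running between 0 and 100 flips the Y direction.
; Only at those flips does it check world X and destroy itself past a negative limit.
; Overlapping a bpBullet sets EnemyHit, which this Blueprint never reads.
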(event EventBeginPlay)

(event Collision|EventActorBeginOverlap
  (params (OtherActor :type Actor%20Object%20Reference))
  (Utilities|Casting|CastTobpBullet OtherActor)
  (Variables|Default|SetEnemyHit true))

(event EventTick
  (params (DeltaSeconds :type Float%20%28single-precision%29))
  (Transformation|AddActorLocalOffset (Math|Vector|MakeVector (|(DeltaSeconds*XMovement) DeltaSeconds (Variables|Default|GetEnemyMovementSpeed)) 0.0 0.0) false false)
  (if (Variables|Default|GetPositiveYMovement)
    (bind _output_get (Variables|Default|SetYMovementDirection 1e+02))
    (Transformation|AddActorLocalOffset (Math|Vector|MakeVector 0.0 (|(DeltaSeconds*YMovement) DeltaSeconds _output_get) 0.0) false false)
    (bind _result (Math|Float|IncrementFloat (Variables|Default|GetTotalYMovement))
      (:%20%20
        (Math|Float|CompareFloat _result 1e+02
          (:==
            (Variables|Default|SetPositiveYMovement false)))))
    (else
      (bind _output_get_2 (Variables|Default|SetYMovementDirection -1e+02))
      (Transformation|AddActorLocalOffset (Math|Vector|MakeVector 0.0 (|(DeltaSeconds*YMovement) DeltaSeconds _output_get_2) 0.0) false false)
      (bind _result_2 (Math|Float|DecrementFloat (Variables|Default|GetTotalYMovement))
        (:%20%20
          (Math|Float|CompareFloat _result_2 0.0
            (:==
              (Variables|Default|SetPositiveYMovement true)))))))
  (Math|Float|CompareFloat (.x (Transformation|GetActorLocation)) -5e+02
    (:<
      (Actor|DestroyActor))))

(fn ConstructionScript)